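; Elevator actor that rises once a Character overlaps its Trigger.
; The overlap latches IsPlayerOn, which nothing resets, and Tick then raises the actor along Z at Speed, without sweep, until it passes the world-space MaxHeight.
; The construction script stores the actor's location as Destination, which only an unused distance-threshold check reads.
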(event OnComponentBeginOverlap(Trigger)
  (params (OverlappedComponent :type Primitive%20Component%20Object%20Reference) (OtherActor :type Actor%20Object%20Reference) (OtherComp :type Primitive%20Component%20Object%20Reference) (OtherBodyIndex :type Integer) (bFromSweep :type Boolean) (SweepResult :type Hit%20Result%20Structure%20%28by%20ref%29))
  (Utilities|Casting|CastToCharacter OtherActor)
  (Variables|Elevator|SetIsPlayerOn true))

(event EventTick
  (params (DeltaSeconds :type Float%20%28single-precision%29))
  (bind _returnvalue (Transformation|GetActorLocation))
  (bind (_x _y _z) (Math|Vector|BreakVector _returnvalue))
  (if (and (Variables|Elevator|GetIsPlayerOn) (>= (Variables|Elevator|GetMaxHeight) _z)) ; Should move?
    (Transformation|SetActorLocation (Math|Vector|MakeVector _x _y (+ _z (* DeltaSeconds (Variables|Elevator|GetSpeed)))) false false) ; Move
  ))

(fn ConstructionScript
  (Variables|Elevator|SetDestination (Transformation|GetActorLocation)))