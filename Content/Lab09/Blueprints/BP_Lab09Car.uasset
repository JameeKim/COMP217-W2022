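; BP_Lab09Car is a lab car actor that moves in a straight line toward a TargetLocation actor.
; Each Tick, while the target is valid, it steps along the normalized direction by Speed times delta time, keeping movement frame-rate independent.
; When the remaining distance is no more than one step, it snaps exactly onto the target to avoid overshooting.
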(event EventTick
  (params (DeltaSeconds :type Float%20%28single-precision%29))
  (bind _returnvalue (Transformation|GetActorLocation))
  (bind _targetlocation (Variables|Car|GetTargetLocation))
  (bind _returnvalue_2 (Transformation|GetActorLocation _targetlocation))
  (bind _returnvalue_3 (- _returnvalue_2 _returnvalue))
  (Utilities|IsValid (Variables|Car|GetTargetLocation)
    (:Is%20Valid
      (if (> (Math|Vector|VectorLength _returnvalue_3) (* DeltaSeconds (Variables|Car|GetSpeed)))
        ;[1 1 1] Move towards the target
        (Transformation|SetActorLocation (+ (Transformation|GetActorLocation) (* (Math|Vector|Normalize _returnvalue_3 0.01) (* (Variables|Car|GetSpeed) DeltaSeconds))) false false)
        (else
          (Transformation|SetActorLocation _returnvalue_2 false false))))))

(fn ConstructionScript)