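; BP_Lab09CarSwitch is a trigger switch that moves a referenced Car and recolors its lights when the player steps in or out.
; Player overlap sets the Car's TargetLocation to EndLocation and the lights to EndColor; leaving restores the start values.
; SetLightColor applies one color to four point lights, and the construction script uses it to show StartColor initially.
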(event OnComponentBeginOverlap(Trigger)
  (params (OverlappedComponent :type Primitive%20Component%20Object%20Reference) (OtherActor :type Actor%20Object%20Reference) (OtherComp :type Primitive%20Component%20Object%20Reference) (OtherBodyIndex :type Integer) (bFromSweep :type Boolean) (SweepResult :type Hit%20Result%20Structure%20%28by%20ref%29))
  (if (== OtherActor (Game|GetPlayerCharacter 0))
    (Variables|/Game/Lab09/Blueprints/BP_Lab09Car.BP_Lab09Car_C|SetTargetLocation (Variables|Car|GetCar) (Variables|Car|GetEndLocation))
    (CallFunction|SetLightColor (Variables|Switch|GetEndColor))))

(event OnComponentEndOverlap(Trigger)
  (params (OverlappedComponent :type Primitive%20Component%20Object%20Reference) (OtherActor :type Actor%20Object%20Reference) (OtherComp :type Primitive%20Component%20Object%20Reference) (OtherBodyIndex :type Integer))
  (if (== OtherActor (Game|GetPlayerCharacter 0))
    (Variables|/Game/Lab09/Blueprints/BP_Lab09Car.BP_Lab09Car_C|SetTargetLocation (Variables|Car|GetCar) (Variables|Car|GetStartLocation))
    (CallFunction|SetLightColor (Variables|Switch|GetStartColor))))

(fn ConstructionScript
  (CallFunction|SetLightColor (Variables|Switch|GetStartColor)))

(fn SetLightColor
  (params (Color :type Linear%20Color%20Structure))
  (Utilities|FlowControl|Sequence
    (:then_0
      (Rendering|Components|Light|SetLightColor (Variables|Default|GetPointLight) Color true))
    (:then_1
      (Rendering|Components|Light|SetLightColor (Variables|Default|GetPointLight1) Color true))
    (:then_2
      (Rendering|Components|Light|SetLightColor (Variables|Default|GetPointLight2) Color true))
    (:then_3
      (Rendering|Components|Light|SetLightColor (Variables|Default|GetPointLight3) Color true))))